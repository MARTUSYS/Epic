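; Player pawn for a tunnel flyer that moves forward with steadily increasing speed and strafes on two input axes.
; BeginPlay creates the HUD and chains initial Tunnel segments through each SpawnPoint, scattering random coins, boosts, bombs and slowdowns.
; Overlaps are resolved by casting: coins update the HUD and material alpha, boosts raise flight speed, slowdowns temporarily cut strafe speed.
; Bombs are destroyed and open NewMap.
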(event `self.ReceiveActorBeginOverlap`
  (params (OtherActor :type "Actor Object Reference"))
  (bind _isvalid (`self.CastToBoo` OtherActor))
  (if _isvalid
    (`self.K2_DestroyActor` OtherActor)
    (`GameplayStatics.OpenLevel` "NewMap")))

(event `self.ReceiveBeginPlay`
  (bind _returnvalue (`PrimitiveComponent.CreateDynamicMaterialInstance` (`self.PlayerRoot`) 0 "/Game/Materials/Corably.Corably" "None"))
  (set `self.NewVar_0` _returnvalue)
  (bind _returnvalue_2 (`|GenericCreateObject` "/Game/Blueprints/HUD.HUD_C" self))
  (bind _output_get (set `self.Hud_val` _returnvalue_2))
  (`UserWidget.AddToViewport` _output_get 0)
  (set `self.Coin_global` 0)
  (for _ (range 5)
    (`/Engine/EditorBlueprintResources/StandardMacros.IsValid` (`self.LastSpawn`)
      (:`Is Valid`
        (`self.SpawnNext`))
      (:`Is Not Valid`
        (`self.SpawnTunnel` (0.0 0.0 0.0))))))

(event `self.ReceiveTick`
  (params (DeltaSeconds :type "Float (single-precision)"))
  (bind _returnvalue (`self.ConsumeMovementInputVector`))
  (`SceneComponent.K2_AddLocalOffset` (`self.PlayerRoot`) (+ (* _returnvalue (* DeltaSeconds (`self.StrafeSpeed`))) (* (`self.GetActorForwardVector`) (* DeltaSeconds (`self.FlightSpeed`)))) true false)
  (set `self.FlightSpeed` (+ (`self.FlightSpeed`) (* DeltaSeconds (`self.acceleration`))))
  (if (`self.slow`)
    (`KismetSystemLibrary.Delay` 3.0)
    (set `self.StrafeSpeed` 100.0)
    (set `self.slow` false)))

(event `InputAxis|AxisX`
  (params (AxisValue :type "Float (single-precision)"))
  (`self.AddMovementInput` (`self.GetActorRightVector`) AxisValue))

(event `InputAxis|AxisY`
  (params (AxisValue :type "Float (single-precision)"))
  (`self.AddMovementInput` (`self.GetActorUpVector`) AxisValue))

(fn `CastToBoo`
  (params (Object :type "Actor Object Reference"))
  (returns (IsValid :type Boolean))
  (cast `/Game/Blueprints/coin` Object
    (:`then`
      (bind _result (`/Engine/EditorBlueprintResources/StandardMacros.IncrementInt` (`self.Coin_global`))
        (:`  `
          (bind _output_get (set `self.Coin_global` _result))
          (bind _alpha_2 (`self.Color` _output_get))
          (`MaterialInstanceDynamic.SetScalarParameterValue` (`self.NewVar_0`) "Alpha" _alpha_2)
          (`self.SetColtext` _output_get))))
    (:`CastFailed`
      (cast `/Game/Blueprints/boost` Object
        (:`then`
          (set `self.FlightSpeed` (* (`self.FlightSpeed`) 1.35)))
        (:`CastFailed`
          (cast `/Game/Blueprints/bomb` Object
            (:`then`
              (return true))
            (:`CastFailed`
              (cast `/Game/Blueprints/slowdown` Object)
              (set `self.StrafeSpeed` (* (`self.StrafeSpeed`) 0.5))
              (set `self.slow` true)))))))
  (return false))

(fn `Color`
  (params (Coin :type Integer))
  (returns (Alpha_2 :type "Float (double-precision)"))
  (`/Engine/EditorBlueprintResources/StandardMacros.CompareInt` Coin 5
    (:`>`
      _)
    (:`==`
      _)
    (:`<`
      (return (/ (`KismetMathLibrary.Conv_IntToDouble` Coin) 5.0))))
  (return 1.0))

(fn `OnRep_NewVar_0`)

(fn `SetColtext`
  (params (coin :type Integer))
  (`TextBlock.SetText` (`/Game/Blueprints/HUD.Coin_val` (`self.Hud_val`)) (`KismetTextLibrary.Conv_IntToText` coin)))

(fn `SpawnNext`
  (bind _returnvalue (`SceneComponent.K2_GetComponentLocation` (`/Game/Blueprints/tunnel.SpawnPoint` (`self.LastSpawn`))))
  (`self.SpawnTunnel` _returnvalue)
  (`self.SpawnRandomBoost` _returnvalue))

(fn `SpawnRandomBoost`
  (params (Loc :type "Vector Structure"))
  (bind _returnvalue (`KismetMathLibrary.MakeVector` (`KismetMathLibrary.RandomFloatInRange` 1.0 4.0) (`KismetMathLibrary.RandomFloatInRange` 1.0 4.0) (`KismetMathLibrary.RandomFloatInRange` 1.0 4.0)))
  (bind _returnvalue_2 (+ Loc (`KismetMathLibrary.MakeVector` (`KismetMathLibrary.RandomFloatInRange` 10.0 50.0) (`KismetMathLibrary.RandomFloatInRange` -50.0 50.0) (`KismetMathLibrary.RandomFloatInRange` -50.0 50.0))))
  (switch `int` (`KismetMathLibrary.RandomInteger` 4)
    (:`Default`
      (`|SpawnActorFromClass` "/Game/Blueprints/slowdown.slowdown_C" (`KismetMathLibrary.MakeTransform` _returnvalue_2 (struct) _returnvalue) "Undefined" "OverrideRootScale" null null :!label _label))
    (:`0`
      (`|SpawnActorFromClass` "/Game/Blueprints/bomb.bomb_C" (`KismetMathLibrary.MakeTransform` _returnvalue_2 (struct) _returnvalue) "Undefined" "OverrideRootScale" null null))
    (:`1`
      (`|SpawnActorFromClass` "/Game/Blueprints/boost.boost_C" (`KismetMathLibrary.MakeTransform` _returnvalue_2 (struct) _returnvalue) "Undefined" "OverrideRootScale" null null))
    (:`2`
      (`|SpawnActorFromClass` "/Game/Blueprints/coin.coin_C" (`KismetMathLibrary.MakeTransform` _returnvalue_2 (struct) _returnvalue) "Undefined" "OverrideRootScale" null null))
    (:`3`
      (goto _label))))

(fn `SpawnTunnel`
  (params (Loc :type "Vector Structure"))
  (bind _returnvalue (`|SpawnActorFromClass` "/Game/Blueprints/tunnel.tunnel_C" (`KismetMathLibrary.MakeTransform` Loc) "Undefined" "OverrideRootScale" null null))
  (set `self.LastSpawn` _returnvalue))

(fn `UserConstructionScript`)